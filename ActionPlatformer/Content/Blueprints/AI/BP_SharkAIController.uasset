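; AI controller for the shark enemy, driving BP_Shark with the BT_Shark behavior tree on the BB_Shark blackboard.
; On possession it starts the tree and stores the shark's current location as its home in the blackboard.
; It listens to the shark's stun-state event and mirrors it into a blackboard flag for the tree to use.
; A StopAI helper halts the brain's logic.
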(event `self.ReceivePossess`
  (params (PossessedPawn :type "Pawn Object Reference"))
  (bind _asbp_shark (cast `/Game/Blueprints/Characters/BP_Shark` PossessedPawn))
  (set `self.OwningCharacter` _asbp_shark)
  (`self.RunAI`)
  (`BlackboardComponent.SetValueAsVector` (`self.Blackboard`) (`self.HomeKeyName`) (`self.K2_GetActorLocation` (`self.OwningCharacter`)))
  (add `/Game/Blueprints/Characters/BP_ActionChar.OnStunStateChanged` (`self.OwningCharacter`) (delegate `StunStateChanged`)))

(event `StunStateChanged`
  (params (InIsStunned :type Boolean))
  (`BlackboardComponent.SetValueAsBool` (`self.Blackboard`) (`self.IsStunnedKeyName`) InIsStunned))

(fn `RunAI`
  (bind (_blackboardcomponent _returnvalue) (`self.UseBlackboard` "/Game/AI/BB_Shark.BB_Shark"))
  (if _returnvalue
    (`self.RunBehaviorTree` "/Game/AI/BT_Shark.BT_Shark")))

(fn `StopAI`
  (`BrainComponent.StopLogic` (`self.BrainComponent`) ""))

(fn `UserConstructionScript`)