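; BP_APGameMode is a game mode that spawns enemies over time and presents the match result.
; On BeginPlay it caches every TargetPoint as a spawn point and starts a timer.
; SpawnEnemy spawns at a random cached point, ignoring collisions, then sets another timer with a random delay.
; SetGameResult disables player input and shows the WBP_GameResult widget with the success or failure outcome.
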(event `self.ReceiveBeginPlay`
  (bind _outactors (`GameplayStatics.GetAllActorsOfClass` "/Script/Engine.TargetPoint"))
  (set `self.SpawnPoints` _outactors)
  (`KismetSystemLibrary.K2_SetTimerDelegate` (`|CreateDelegate` :!event `SpawnEnemy`) 5.0))

(fn `SetGameResult`
  (params (IsSuccess :type Boolean))
  (bind _returnvalue (`GameplayStatics.GetPlayerController` 0))
  (`self.DisableInput` _returnvalue null)
  (bind _returnvalue_2 (`|CreateWidget` "/Game/Paper2DAssets/UI/WBP_GameResult.WBP_GameResult_C" _returnvalue))
  (`UserWidget.AddToViewport` _returnvalue_2 0)
  (`/Game/Paper2DAssets/UI/WBP_GameResult.SetResult` _returnvalue_2 (`local.IsSuccess`)))

(fn `SpawnEnemy`
  (`|SpawnActorFromClass` "/Game/Blueprints/Characters/BP_Shark.BP_Shark_C" (`self.GetTransform` (`|GetArrayItem` (`self.SpawnPoints`) (`KismetMathLibrary.RandomIntegerInRange` 0 (- (`KismetArrayLibrary.Array_Length` (`self.SpawnPoints`)) 1)))) "AlwaysSpawn" "MultiplyWithRoot" null null)
  (`KismetSystemLibrary.K2_SetTimerDelegate` (`|CreateDelegate` :!event `SpawnEnemy`) (`KismetMathLibrary.RandomFloatInRange` 3.0 10.0)))

(fn `UserConstructionScript`)