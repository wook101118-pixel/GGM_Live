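; BP_Shark is an AI-controlled shark character that handles its own death and facing on top of its parent class.
; Every tick, SetFocusDirection points the AI focal point along the X velocity while it can act and is moving, otherwise along its forward vector.
; Using only X keeps the focus target horizontal along that single axis.
; On death, it stops its BP_SharkAIController and destroys itself after a short delay.
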(event `self.ReceiveBeginPlay`
  (`parent.ReceiveBeginPlay`)
  (add `self.OnDead` (delegate `OnSharkDead`)))

(event `OnSharkDead`
  (bind _asbp_shark_aicontroller (cast `/Game/Blueprints/AI/BP_SharkAIController` (`AIBlueprintHelperLibrary.GetAIController` self)))
  (`/Game/Blueprints/AI/BP_SharkAIController.StopAI` _asbp_shark_aicontroller)
  (`KismetSystemLibrary.Delay` 2.0)
  (`self.K2_DestroyActor`))

(event `self.ReceiveTick`
  (params (DeltaSeconds :type "Float (single-precision)"))
  (`parent.ReceiveTick` DeltaSeconds)
  (`self.SetFocusDirection`))

(fn `SetFocusDirection`
  (bind _returnvalue_x (`KismetMathLibrary.BreakVector` (`self.GetVelocity`)))
  (if (and (`self.CanAct`) (`KismetMathLibrary.NotEqualExactly_VectorVector` (`self.GetVelocity`)))
    (bind _asaicontroller (cast `AIController` (`self.GetController`)))
    (`AIController.K2_SetFocalPoint` _asaicontroller (+ (`self.K2_GetActorLocation`) (`KismetMathLibrary.MakeVector` _returnvalue_x)))
    (else
      (bind _asaicontroller_2 (cast `AIController` (`self.GetController`)))
      (`AIController.K2_SetFocalPoint` _asaicontroller_2 (+ (`self.K2_GetActorLocation`) (`self.GetActorForwardVector`))))))

(fn `UserConstructionScript`
  (`parent.UserConstructionScript`))