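; BP_ActionChar is a sprite-based action character that handles melee hits, health, stun and death.
; Its toggleable HitBox damages other overlapped BP_ActionChars and triggers hit stop on both by zeroing CustomTimeDilation behind a retriggerable delay.
; ReceiveAttack either kills or stuns, firing dispatchers and jumping animation states, with timers for stun length and sprite shake.
; CanAct gates actions on attacking, stunned and dead flags.
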(event `self.ReceiveBeginPlay`
  (`self.SetHitBoxCollision` false)
  (set `self.CurrentHealth` (`self.MaxHealth`))
  (set `self.SpriteBaseLocation` (`SceneComponent.RelativeLocation` (`self.Sprite`))))

(event `self.HitBox.OnComponentBeginOverlap`
  (params (OverlappedComponent :type "PrimitiveComponent Object Reference") (OtherActor :type "Actor Object Reference") (OtherComp :type "PrimitiveComponent Object Reference") (OtherBodyIndex :type Integer) (bFromSweep :type Boolean) (SweepResult :type "HitResult Structure (by ref)"))
  (if (!= OtherActor self)
    (bind _asbp_action_char (cast `/Game/Blueprints/Characters/BP_ActionChar` OtherActor))
    (`self.ReceiveAttack` _asbp_action_char (`self.HitDamage`))
    (`self.HitStopEvent` _asbp_action_char 0.2)
    (`self.HitStopEvent` 0.2)))

(event `HitStopEvent`
  (params (Duration :type "Float (double-precision)" :default 0.2))
  (set `self.CustomTimeDilation` 0.0)
  (`KismetSystemLibrary.RetriggerableDelay` Duration)
  (set `self.CustomTimeDilation` 1.0))

(fn `CanAct`
  (returns (Result :type Boolean))
  (return (and (not (`self.IsAttacking`)) (not (`self.IsStunned`)) (not (`self.IsDead`)))))

(fn `ClearStun`
  (bind _output_get (set `self.IsStunned` false))
  (`self.OnStunStateChanged` _output_get)
  (`KismetSystemLibrary.K2_ClearAndInvalidateTimerHandle` (`self.SpriteShakeTimer`))
  (`SceneComponent.K2_SetRelativeLocation` (`self.Sprite`) (`self.SpriteBaseLocation`) false false))

(fn `ReceiveAttack`
  (params (InDamage :type "Float (double-precision)"))
  (if (not (`self.IsDead`))
    (`GameplayStatics.PlaySoundAtLocation` "/Game/Paper2DAssets/Sounds/S_Hit_Cue.S_Hit_Cue" (`self.K2_GetActorLocation`) (struct) 1.0 1.0 0.0 null null null null)
    (bind _output_get (set `self.CurrentHealth` (`KismetMathLibrary.FClamp` (- (`self.CurrentHealth`) (`local.InDamage`)) 0.0 (`self.MaxHealth`))))
    (if (<= _output_get 0.0)
      (set `self.IsDead` true)
      (`self.OnDead`)
      (`PaperZDAnimInstance.JumpToNode` (`self.GetAnimInstance`) "JumpDead" "None")
      (`PrimitiveComponent.SetCollisionEnabled` (`self.CapsuleComponent`) "NoCollision")
      (else
        (bind _output_get_2 (set `self.IsStunned` true))
        (`self.OnStunStateChanged` _output_get_2)
        (`PaperZDAnimInstance.JumpToNode` (`self.GetAnimInstance`) "JumpStunned" "None")
        (`KismetSystemLibrary.K2_SetTimerDelegate` (`|CreateDelegate` :!event `ClearStun`) (`self.StunLength`))
        (bind _returnvalue (`KismetSystemLibrary.K2_SetTimerDelegate` (`|CreateDelegate` :!event `ShakeSprite`) (`self.SpriteShakeFrequency`) true))
        (set `self.SpriteShakeTimer` _returnvalue)))))

(fn `SetHitBoxCollision`
  (params (InActive :type Boolean))
  (if InActive
    (`PrimitiveComponent.SetCollisionEnabled` (`self.HitBox`) "QueryAndPhysics")
    (else
      (`PrimitiveComponent.SetCollisionEnabled` (`self.HitBox`) "NoCollision"))))

(fn `ShakeSprite`
  (bind (_spritebaselocation_x _spritebaselocation_y _spritebaselocation_z) (`KismetMathLibrary.BreakVector` (`self.SpriteBaseLocation`)))
  (bind _isa (`/Engine/EditorBlueprintResources/StandardMacros.FlipFlop`)
    (:`A`
      _)
    (:`B`
      _))
  (`SceneComponent.K2_SetRelativeLocation` (`self.Sprite`) (`KismetMathLibrary.MakeVector` (+ (`KismetMathLibrary.SelectFloat` (* (`self.SpriteShakeDistance`) -1.0) (`self.SpriteShakeDistance`) _isa) _spritebaselocation_x) _spritebaselocation_y _spritebaselocation_z) false false))

(fn `UserConstructionScript`)