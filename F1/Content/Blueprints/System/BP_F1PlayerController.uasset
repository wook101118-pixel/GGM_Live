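; BP_F1PlayerController is a player controller that lets the player cycle control between the pawns in the level.
; On BeginPlay it caches every Pawn actor into the F1PPawns array.
; Pressing Tab calls ChangePawn, which validates the index, unpossesses the current pawn and possesses the one at NextPawnIndex, then advances that index with wraparound.
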(event `self.ReceiveBeginPlay`
  (bind _outactors (`GameplayStatics.GetAllActorsOfClass` "/Script/Engine.Pawn"))
  (set `self.F1PPawns` _outactors))

(event `Key|Tab`
  (params (Key :type "Key Structure"))
  (:`Pressed`
    (`self.ChangePawn` (`self.NextPawnIndex`))
    (set `self.NextPawnIndex` (mod (+ (`self.NextPawnIndex`) 1) (`KismetArrayLibrary.Array_Length` (`self.F1PPawns`))))))

(fn `ChangePawn`
  (params (NewIndex :type Integer))
  (if (`KismetArrayLibrary.Array_IsValidIndex` (`self.F1PPawns`) NewIndex)
    (`self.UnPossess`)
    (`self.Possess` (`|GetArrayItem` (`self.F1PPawns`) (`local.NewIndex`)))))

(fn `UserConstructionScript`)